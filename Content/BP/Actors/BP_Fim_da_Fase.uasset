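; End-of-level trigger actor that opens the "Creditos" level when the player carries the key item, apparently a steering wheel.
; Box overlap, with no check on the overlapping actor, calls VerificarItem, which searches the player's BPCInventory for an item class whose default name matches NomeDoItemChave.
; A match sets FimdaFase on the L1_Horror_Character; otherwise a debug message requests the item.
; The item-removal logic is disconnected.
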(event OnComponentBeginOverlap(Box)
  (params (OverlappedComponent :type Primitive%20Component%20Object%20Reference) (OtherActor :type Actor%20Object%20Reference) (OtherComp :type Primitive%20Component%20Object%20Reference) (OtherBodyIndex :type Integer) (bFromSweep :type Boolean) (SweepResult :type Hit%20Result%20Structure%20%28by%20ref%29))
  (bind _sucess (CallFunction|VerificarItem))
  (if _sucess
    (Development|PrintString "passou")
    (Game|OpenLevel(byName) "Creditos")
    (else
      (Development|PrintString "Tem que pegar o volante"))))

(event EventBeginPlay
  (bind _asl1_horror_character (Utilities|Casting|CastToL1_Horror_Character (Game|GetPlayerCharacter 0)))
  (Variables|Default|SetPlayerCharacterRef _asl1_horror_character))

(event Collision|EventActorBeginOverlap
  (params (OtherActor :type Actor%20Object%20Reference)))

(event EventTick
  (params (DeltaSeconds :type Float%20%28single-precision%29)))

(fn ConstructionScript)

(fn VerificarItem
  (bind (_array_element _array_index) (Utilities|Array|ForEachLoopwithBreak (Variables|/Game/BP/BP_Component/BPC_Inventory.BPC_Inventory_C|GetS_InventoryItem (Variables|/Game/GameBP/Level1/L1_Horror_Character.L1_Horror_Character_C|GetBPC_Inventory (Variables|Default|GetPlayerCharacterRef))) :!label _label)
    (:LoopBody
      (if (Utilities|IsValidClass (.Item (Utilities|Struct|BreakS_InventoryItems _array_element)))
        (if (Utilities|Name|Equal(Name) (.ItemName (Utilities|Struct|BreakS_ItemData (.S_ItemData (Utilities|GetClassDefaults (.Item (Utilities|Struct|BreakS_InventoryItems _array_element)))))) (Variables|Default|GetNome%20do%20item%20chave))
          (Development|PrintString "f")
          (Variables|/Game/GameBP/Level1/L1_Horror_Character.L1_Horror_Character_C|SetFimdaFase (Variables|Default|GetPlayerCharacterRef) true)
          (goto _label Break)
          (else
            _)))
      (Development|PrintString "l"))
    (:Completed
      (if (Variables|/Game/GameBP/Level1/L1_Horror_Character.L1_Horror_Character_C|GetFimdaFase (Variables|Default|GetPlayerCharacterRef))
        (return true)
        (else
          (return false))))))