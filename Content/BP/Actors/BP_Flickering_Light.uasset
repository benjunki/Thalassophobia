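; BP_Flickering_Light is an actor that makes its point light flicker at irregular intervals.
; From BeginPlay it loops endlessly, waiting a random delay between MinTime and MaxTime, then using a FlipFlop to alternate between MinFlickerIntensity and Intensity.
; The construction script does nothing, as its SetIntensity node is not connected.
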(event EventBeginPlay
  (Utilities|FlowControl|RetriggerableDelay (Math|Random|RandomFloatinRange (Variables|Default|GetMin%20time) (Variables|Default|GetMax%20Time)) :!label _label)
  (Utilities|FlowControl|FlipFlop
    (:A
      (Rendering|Components|Light|SetIntensity (Variables|Default|GetPointLight) (Variables|Default|GetMin%20Flicker%20Intensity))
      (goto _label))
    (:B
      (Rendering|Components|Light|SetIntensity (Variables|Default|GetPointLight) (Variables|Default|GetIntensity))
      (goto _label))))

(fn ConstructionScript)