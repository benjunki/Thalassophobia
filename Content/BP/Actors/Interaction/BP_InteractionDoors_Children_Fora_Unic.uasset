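; Interactive hinged door, apparently a child Blueprint, that the player toggles open and closed and that opens automatically for AI_TheClassic.
; Interact drives one timeline and the Box overlap events drive another, both rotating Door's yaw by 90 degrees.
; A dot product between the opener-to-door direction and the door's forward vector picks the swing side.
; AI entry blocks player interaction until the automatic close finishes, and AI exit closes an open door.
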(event OnComponentBeginOverlap(Box)
  (params (OverlappedComponent :type Primitive%20Component%20Object%20Reference) (OtherActor :type Actor%20Object%20Reference) (OtherComp :type Primitive%20Component%20Object%20Reference) (OtherBodyIndex :type Integer) (bFromSweep :type Boolean) (SweepResult :type Hit%20Result%20Structure%20%28by%20ref%29))
  (bind _self self)
  (bind _asai_the_classic (Utilities|Casting|CastToAI_TheClassic OtherActor))
  (Variables|Default|SetCanInteract false)
  (if (not (Variables|Default|GetPortaAberta))
    (Variables|Default|SetPortaAberta true)
    (Variables|Default|SetDot%20Product (Math|Vector|DotProduct (Math|Vector|Normalize (- (Transformation|GetActorLocation _self) (Transformation|GetActorLocation _asai_the_classic))) (Transformation|GetActorForwardVector _self)))
    (bind (_direction _alpha) (Timeline|Timeline_0 PlayFromStart)
      (:Update
        (Transformation|SetRelativeRotation (Variables|Default|GetDoor) (Math|Rotator|MakeRotator 0.0 0.0 (Math|Float|Lerp 0.0 (select (>= (Variables|Default|GetDot%20Product) 0.0) 9e+01 -9e+01) _alpha)) false false))
      (:Finished
        (switch Utilities|FlowControl|Switch|SwitchonETimelineDirection _direction
          (:Backward
            (Variables|Default|SetCanInteract true)))))))

(event OnComponentEndOverlap(Box)
  (params (OverlappedComponent :type Primitive%20Component%20Object%20Reference) (OtherActor :type Actor%20Object%20Reference) (OtherComp :type Primitive%20Component%20Object%20Reference) (OtherBodyIndex :type Integer))
  (Utilities|Casting|CastToAI_TheClassic OtherActor)
  (if (Variables|Default|GetPortaAberta)
    (Variables|Default|SetPortaAberta false)
    (bind (_direction _alpha) (Timeline|Timeline_0 ReverseFromEnd)
      (:Update
        (Transformation|SetRelativeRotation (Variables|Default|GetDoor) (Math|Rotator|MakeRotator 0.0 0.0 (Math|Float|Lerp 0.0 (select (>= (Variables|Default|GetDot%20Product) 0.0) 9e+01 -9e+01) _alpha)) false false))
      (:Finished
        (switch Utilities|FlowControl|Switch|SwitchonETimelineDirection _direction
          (:Backward
            (Variables|Default|SetCanInteract true)))))))

(event EventBeginPlay
  (|CallParentFunction) ; This node is disabled and will not be called.\nDrag off pins to build functionality.
)

(event Collision|EventActorBeginOverlap
  (params (OtherActor :type Actor%20Object%20Reference))
  (|CallParentFunction OtherActor) ; This node is disabled and will not be called.\nDrag off pins to build functionality.
)

(event EventInteract
  (bind _self self)
  (if (Variables|Default|GetCanInteract)
    (if (Variables|Default|GetPortaAberta)
      (Variables|Default|SetPortaAberta false)
      (bind _alpha (Timeline|PortaAbrir ReverseFromEnd)
        (:Update
          (Transformation|SetRelativeRotation (Variables|Default|GetDoor) (Math|Rotator|MakeRotator 0.0 0.0 (Math|Float|Lerp 0.0 (select (>= (Variables|Default|GetDot%20Product) 0.0) 9e+01 -9e+01) _alpha)) false false)))
      (else
        (Variables|Default|SetPortaAberta true)
        (Variables|Default|SetDot%20Product (Math|Vector|DotProduct (Math|Vector|Normalize (- (Transformation|GetActorLocation _self) (Transformation|GetActorLocation (Variables|Default|GetPlayer%20Ref)))) (Transformation|GetActorForwardVector _self)))
        (Timeline|PortaAbrir PlayFromStart)))))

(fn ConstructionScript
  (|CallParentFunction))