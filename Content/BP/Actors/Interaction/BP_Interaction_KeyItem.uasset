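; BP_Interaction_KeyItem is an interactable pickup that gives the player an item, likely a key item, in a horror game.
; On Interact, it casts the player character to L1_Horror_Character and adds its Item and Amount to that character's inventory component.
; The actor destroys itself only when the add succeeds, so a failed add leaves it in the world.
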(event EventBeginPlay
  (|CallParentFunction) ; This node is disabled and will not be called.\nDrag off pins to build functionality.
)

(event Collision|EventActorBeginOverlap
  (params (OtherActor :type Actor%20Object%20Reference))
  (|CallParentFunction OtherActor) ; This node is disabled and will not be called.\nDrag off pins to build functionality.
)

(event EventTick
  (params (DeltaSeconds :type Float%20%28single-precision%29))
  (|CallParentFunction DeltaSeconds) ; This node is disabled and will not be called.\nDrag off pins to build functionality.
)

(event EventInteract
  (bind _asl1_horror_character (Utilities|Casting|CastToL1_Horror_Character (Game|GetPlayerCharacter 0)))
  (bind _sucess (Default|AddItem (Variables|/Game/GameBP/Level1/L1_Horror_Character.L1_Horror_Character_C|GetBPC_Inventory _asl1_horror_character) (Variables|Default|GetItem) (Variables|Default|GetAmount_0)))
  (if _sucess
    (Actor|DestroyActor)))

(fn ConstructionScript
  (|CallParentFunction))