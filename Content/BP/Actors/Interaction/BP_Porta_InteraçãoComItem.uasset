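; Interactable swinging door that can be locked behind a named key item and also opens for AI_TheClassic.
; Interact runs VerificarItem, which removes a matching key and unlocks, but gives up at the first non-matching inventory slot, then toggles the door.
; AI overlap opens and closes unlocked doors on a separate timeline, blocking interaction until fully closed.
; A dot product against the opener's position picks the ±90° swing.
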(event OnComponentBeginOverlap(Box)
  (params (OverlappedComponent :type Primitive%20Component%20Object%20Reference) (OtherActor :type Actor%20Object%20Reference) (OtherComp :type Primitive%20Component%20Object%20Reference) (OtherBodyIndex :type Integer) (bFromSweep :type Boolean) (SweepResult :type Hit%20Result%20Structure%20%28by%20ref%29))
  (bind _self self)
  (bind _asai_the_classic (Utilities|Casting|CastToAI_TheClassic OtherActor))
  (if (not (Variables|Default|GetTrancada))
    (Variables|Default|SetCanInteract false)
    (Development|PrintString "deveria abrir")
    (if (not (Variables|Default|GetPortaAberta))
      (Variables|Default|SetPortaAberta true)
      (Variables|Default|SetDot%20Product (Math|Vector|DotProduct (Math|Vector|Normalize (- (Transformation|GetActorLocation _self) (Transformation|GetActorLocation _asai_the_classic))) (Transformation|GetActorForwardVector _self)))
      (bind (_direction _alpha) (Timeline|Timeline_1 PlayFromStart)
        (:Update
          (Transformation|SetRelativeRotation (Variables|Default|Getporta) (Math|Rotator|MakeRotator 0.0 0.0 (Math|Float|Lerp 0.0 (select (>= (Variables|Default|GetDot%20Product) 0.0) 9e+01 -9e+01) _alpha)) false false))
        (:Finished
          (switch Utilities|FlowControl|Switch|SwitchonETimelineDirection _direction
            (:Backward
              (Variables|Default|SetCanInteract true))))))))

(event OnComponentEndOverlap(Box)
  (params (OverlappedComponent :type Primitive%20Component%20Object%20Reference) (OtherActor :type Actor%20Object%20Reference) (OtherComp :type Primitive%20Component%20Object%20Reference) (OtherBodyIndex :type Integer))
  (Utilities|Casting|CastToAI_TheClassic OtherActor)
  (if (not (Variables|Default|GetTrancada))
    (if (Variables|Default|GetPortaAberta)
      (Variables|Default|SetPortaAberta false)
      (bind (_direction _alpha) (Timeline|Timeline_1 ReverseFromEnd)
        (:Update
          (Transformation|SetRelativeRotation (Variables|Default|Getporta) (Math|Rotator|MakeRotator 0.0 0.0 (Math|Float|Lerp 0.0 (select (>= (Variables|Default|GetDot%20Product) 0.0) 9e+01 -9e+01) _alpha)) false false))
        (:Finished
          (switch Utilities|FlowControl|Switch|SwitchonETimelineDirection _direction
            (:Backward
              (Variables|Default|SetCanInteract true))))))))

(event EventInteract
  (bind _self self)
  (CallFunction|VerificarItem)
  (if (Variables|Default|GetCanInteract)
    (if (not (Variables|Default|GetTrancada))
      (if (Variables|Default|GetPortaAberta)
        (Variables|Default|SetPortaAberta false)
        (bind _alpha (Timeline|Timeline_0 ReverseFromEnd)
          (:Update
            (Transformation|SetRelativeRotation (Variables|Default|Getporta) (Math|Rotator|MakeRotator 0.0 0.0 (Math|Float|Lerp 0.0 (select (>= (Variables|Default|GetDot%20Product) 0.0) 9e+01 -9e+01) _alpha)) false false)))
        (else
          (Variables|Default|SetPortaAberta true)
          (Variables|Default|SetDot%20Product (Math|Vector|DotProduct (Math|Vector|Normalize (- (Transformation|GetActorLocation _self) (Transformation|GetActorLocation (Variables|Default|GetPlayer%20Ref)))) (Transformation|GetActorForwardVector _self)))
          (Timeline|Timeline_0 PlayFromStart))))))

(fn ConstructionScript
  (|CallParentFunction))

(fn VerificarItem
  (bind (_array_element _array_index) (Utilities|Array|ForEachLoopwithBreak (Variables|/Game/BP/BP_Component/BPC_Inventory.BPC_Inventory_C|GetS_InventoryItem (Variables|/Game/GameBP/Level1/L1_Horror_Character.L1_Horror_Character_C|GetBPC_Inventory (Variables|Default|GetPlayer%20Ref))) :!label _label)
    (:LoopBody
      (if (Utilities|IsValidClass (.Item (Utilities|Struct|BreakS_InventoryItems _array_element)))
        (if (Utilities|Name|Equal(Name) (.ItemName (Utilities|Struct|BreakS_ItemData (.S_ItemData (Utilities|GetClassDefaults (.Item (Utilities|Struct|BreakS_InventoryItems _array_element)))))) (Variables|Default|GetNome%20do%20item%20chave))
          (goto _label Break)
          (else
            _)))
      (return))
    (:Completed
      (bind _output_get (LocalVariables|SetLocalSlotIndex _array_index))
      (Default|RemoveItem (Variables|/Game/GameBP/Level1/L1_Horror_Character.L1_Horror_Character_C|GetBPC_Inventory (Variables|Default|GetPlayer%20Ref)) _output_get)
      (Variables|Default|SetTrancada false)
      (return))))