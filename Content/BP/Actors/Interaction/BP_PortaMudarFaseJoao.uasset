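; BP_PortaMudarFaseJoao is an interactable door that moves the player to the next level, Andar2.
; BeginPlay caches the player as an L1_Horror_Character.
; Interact only works while that character's GeradorEstaFuncionando (generator running) flag is true.
; A CanInteract flag then blocks repeat use, and the level opens by name after a short delay.
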(event EventBeginPlay
  (bind _asl1_horror_character (Utilities|Casting|CastToL1_Horror_Character (Game|GetPlayerCharacter 0)))
  (Variables|Default|SetPlayerCharacterRef _asl1_horror_character))

(event Collision|EventActorBeginOverlap
  (params (OtherActor :type Actor%20Object%20Reference)))

(event EventTick
  (params (DeltaSeconds :type Float%20%28single-precision%29)))

(event EventInteract
  (if (Variables|/Game/GameBP/Level1/L1_Horror_Character.L1_Horror_Character_C|GetGeradorEstaFuncionando (Variables|Default|GetPlayerCharacterRef))
    (if (Variables|Default|GetCanInteract)
      (Variables|Default|SetCanInteract false)
      (Utilities|FlowControl|Delay 1.0)
      (Game|OpenLevel(byName) "Andar2"))))

(fn ConstructionScript)