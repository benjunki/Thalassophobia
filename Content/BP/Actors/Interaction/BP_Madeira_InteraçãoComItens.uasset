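; Interactable wood actor (Madeira) that requires a key item from the player's inventory and destroys itself when used.
; On Interact, VerificarItem scans the inventory slots for an item whose class-default name matches NomeDoItemChave, setting the player's PodeMudarDeFase (can change level) flag on a match.
; Success depends on that player flag, which triggers removal of the item at the loop index, disabling of interaction and destruction of the actor.
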(event EventBeginPlay
  (|CallParentFunction) ; This node is disabled and will not be called.\nDrag off pins to build functionality.
)

(event Collision|EventActorBeginOverlap
  (params (OtherActor :type Actor%20Object%20Reference))
  (|CallParentFunction OtherActor) ; This node is disabled and will not be called.\nDrag off pins to build functionality.
)

(event EventTick
  (params (DeltaSeconds :type Float%20%28single-precision%29))
  (|CallParentFunction DeltaSeconds) ; This node is disabled and will not be called.\nDrag off pins to build functionality.
)

(event EventInteract
  (if (Variables|Default|Getcan%20interact)
    (bind _sucess (CallFunction|VerificarItem))
    (if _sucess
      (Variables|Default|Setcan%20interact false)
      (Actor|DestroyActor))))

(fn ConstructionScript
  (|CallParentFunction))

(fn VerificarItem
  (bind (_array_element _array_index) (Utilities|Array|ForEachLoopwithBreak (Variables|/Game/BP/BP_Component/BPC_Inventory.BPC_Inventory_C|GetS_InventoryItem (Variables|/Game/GameBP/Level1/L1_Horror_Character.L1_Horror_Character_C|GetBPC_Inventory (Variables|Default|GetPlayer%20Ref))) :!label _label)
    (:LoopBody
      (if (Utilities|IsValidClass (.Item (Utilities|Struct|BreakS_InventoryItems _array_element)))
        (if (Utilities|Name|Equal(Name) (.ItemName (Utilities|Struct|BreakS_ItemData (.S_ItemData (Utilities|GetClassDefaults (.Item (Utilities|Struct|BreakS_InventoryItems _array_element)))))) (Variables|Default|GetNome%20do%20item%20chave))
          (Development|PrintString "f")
          (Variables|/Game/GameBP/Level1/L1_Horror_Character.L1_Horror_Character_C|SetPodeMudarDeFase (Variables|Default|GetPlayer%20Ref) true)
          (goto _label Break)
          (else
            _)))
      (Development|PrintString "l"))
    (:Completed
      (if (Variables|/Game/GameBP/Level1/L1_Horror_Character.L1_Horror_Character_C|GetPodeMudarDeFase (Variables|Default|GetPlayer%20Ref))
        (bind _output_get (LocalVariables|SetLocalSlotIndex _array_index))
        (Default|RemoveItem (Variables|/Game/GameBP/Level1/L1_Horror_Character.L1_Horror_Character_C|GetBPC_Inventory (Variables|Default|GetPlayer%20Ref)) _output_get)
        (return true)
        (else
          (return false))))))