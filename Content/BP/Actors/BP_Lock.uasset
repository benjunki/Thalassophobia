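; BP_Lock is a four-dial combination lock actor that opens when the dials match its stored code.
; On BeginPlay it enables player input, then spawns indexed BP_LockDial actors attached to bone sockets on the lock mesh.
; H, J, K and L each rotate one dial, then share a retriggerable delay before CheckCode compares dial numbers to LockCombination.
; A full match plays the LockOpen animation.
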(event EventBeginPlay
  (bind _ashorror_player_controller (Utilities|Casting|CastToHorror_PlayerController (Game|GetPlayerController 0)))
  (bind _output_get (Variables|Default|SetplayerController%20REf _ashorror_player_controller))
  (Input|EnableInput _output_get)
  (for _index (range 0 3)
    (bind _returnvalue (Game|SpawnActorfromClass "/Game/BP/Actors/BP_LockDial.BP_LockDial_C" (Math|Transform|MakeTransform "0, 0, 0" "0, 0, 0" "1,1.000000,1") "AlwaysSpawn" 0 _index 0))
    (Utilities|Array|Add (Variables|Default|GetDials) _returnvalue)
    (Transformation|AttachComponentToComponent _returnvalue (Variables|Default|GetLock) (Utilities|Select :Index _index :Option%200 "DialBone1Socket" :Option%201 "DialBone2Socket" :Option%202 "DialBone3Socket" :Option%203 "DialBone4Socket") "SnapToTarget" "KeepWorld" "KeepWorld" true)))

(event Input|KeyboardEvents|H
  (params (Key :type Key%20Structure :default "None"))
  (:Pressed
    (Default|RotateDial (Utilities|Array|Get(acopy) (Variables|Default|GetDials)))
    (Utilities|FlowControl|RetriggerableDelay 0.5)
    (bind _sucess (CallFunction|CheckCode))
    (if _sucess
      (Components|Animation|PlayAnimation (Variables|Default|GetLock) "/Game/Props/Animation/LockOpen.LockOpen" false))))

(event Input|KeyboardEvents|J
  (params (Key :type Key%20Structure :default "None"))
  (:Pressed
    (Default|RotateDial (Utilities|Array|Get(acopy) (Variables|Default|GetDials) 1))
    (Utilities|FlowControl|RetriggerableDelay 0.5)
    (bind _sucess (CallFunction|CheckCode))
    (if _sucess
      (Components|Animation|PlayAnimation (Variables|Default|GetLock) "/Game/Props/Animation/LockOpen.LockOpen" false))))

(event Input|KeyboardEvents|K
  (params (Key :type Key%20Structure :default "None"))
  (:Pressed
    (Default|RotateDial (Utilities|Array|Get(acopy) (Variables|Default|GetDials) 2))
    (Utilities|FlowControl|RetriggerableDelay 0.5)
    (bind _sucess (CallFunction|CheckCode))
    (if _sucess
      (Components|Animation|PlayAnimation (Variables|Default|GetLock) "/Game/Props/Animation/LockOpen.LockOpen" false))))

(event Input|KeyboardEvents|L
  (params (Key :type Key%20Structure :default "None"))
  (:Pressed
    (Default|RotateDial (Utilities|Array|Get(acopy) (Variables|Default|GetDials) 3))
    (Utilities|FlowControl|RetriggerableDelay 0.5)
    (bind _sucess (CallFunction|CheckCode))
    (if _sucess
      (Components|Animation|PlayAnimation (Variables|Default|GetLock) "/Game/Props/Animation/LockOpen.LockOpen" false))))

(fn ConstructionScript)

(fn CheckCode
  (bind (_array_element _array_index) (Utilities|Array|ForEachLoopwithBreak (Variables|Default|GetDials) :!label _label)
    (:LoopBody
      (if (== (Variables|/Game/BP/Actors/BP_LockDial.BP_LockDial_C|GetNumber _array_element) (Utilities|Array|Get(acopy) (Variables|Default|GetlockCombination) _array_index))
        (LocalVariables|SetLocalSucess true)
        (else
          (LocalVariables|SetLocalSucess false)
          (goto _label Break))))
    (:Completed
      (return (LocalVariables|GetLocalSucess)))))