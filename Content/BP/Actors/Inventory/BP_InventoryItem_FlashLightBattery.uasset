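; An inventory item Blueprint for a flashlight battery that recharges the player's flashlight when used.
; UseItem checks the flashlight component on the player reference, and if CurrentBattery is below MaxBattery it calls AddBatteryLife with BatteryAmount.
; UseItemSucess records whether the charge was applied, so use fails when the battery is already full.
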(event EventBeginPlay
  (|CallParentFunction) ; This node is disabled and will not be called.\nDrag off pins to build functionality.
)

(event Collision|EventActorBeginOverlap
  (params (OtherActor :type Actor%20Object%20Reference))
  (|CallParentFunction OtherActor) ; This node is disabled and will not be called.\nDrag off pins to build functionality.
)

(event EventTick
  (params (DeltaSeconds :type Float%20%28single-precision%29))
  (|CallParentFunction DeltaSeconds) ; This node is disabled and will not be called.\nDrag off pins to build functionality.
)

(event EventUseItem
  (bind _playerref (Variables|Default|GetPlayerRef))
  (bind _bpc_flashlight (Variables|/Game/GameBP/Level1/L1_Horror_Character.L1_Horror_Character_C|GetBPC_FlashLight _playerref))
  (if (< (Variables|/Game/BP/BP_Component/BPC_FlashLight.BPC_FlashLight_C|GetCurrentBattery _bpc_flashlight) (Variables|/Game/BP/BP_Component/BPC_FlashLight.BPC_FlashLight_C|GetMaxBattery _bpc_flashlight))
    (Default|AddBatteryLife _bpc_flashlight (Variables|Default|GetBatteryAmount))
    (Variables|Default|SetUseItemSucess true)
    (else
      (Variables|Default|SetUseItemSucess false))))

(fn ConstructionScript
  (|CallParentFunction))