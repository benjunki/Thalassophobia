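; Master note actor for a horror game that shows a pickup prompt and opens an examine widget.
; Sphere overlap starts a per-tick visibility trace to the player camera, hiding the prompt and disabling input when blocked.
; Otherwise the prompt faces the camera, and pickup distance toggles its state and input.
; The action key creates the examine widget, linked to the level's BP_Note_Examination; construction fills front and back text.
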(event OnComponentBeginOverlap(Sphere)
  (params (OverlappedComponent :type Primitive%20Component%20Object%20Reference) (OtherActor :type Actor%20Object%20Reference) (OtherComp :type Primitive%20Component%20Object%20Reference) (OtherBodyIndex :type Integer) (bFromSweep :type Boolean) (SweepResult :type Hit%20Result%20Structure%20%28by%20ref%29))
  (bind _asl1_horror_character (Utilities|Casting|CastToL1_Horror_Character OtherActor))
  (Variables|Default|SetPlayerREf _asl1_horror_character)
  (Rendering|SetVisibility (Variables|Default|GetPromptWidget) true false)
  (Variables|Default|SetUpdateActor true))

(event OnComponentEndOverlap(Sphere)
  (params (OverlappedComponent :type Primitive%20Component%20Object%20Reference) (OtherActor :type Actor%20Object%20Reference) (OtherComp :type Primitive%20Component%20Object%20Reference) (OtherBodyIndex :type Integer))
  (Utilities|Casting|CastToL1_Horror_Character OtherActor)
  (Rendering|SetVisibility (Variables|Default|GetPromptWidget) false false)
  (Variables|Default|SetUpdateActor false)
  (Input|DisableInput (Game|GetPlayerController 0)))

(event EventTick
  (params (DeltaSeconds :type Float%20%28single-precision%29))
  (bind _returnvalue (Game|GetPlayerController 0))
  (bind _promptwidget (Variables|Default|GetPromptWidget))
  (bind _papermesh (Variables|Default|GetPaperMesh))
  (bind _returnvalue_2 (Transformation|GetWorldLocation _papermesh))
  (Transformation|SetWorldLocation (Variables|Default|GetPromptWidget) (Math|Vector|MakeVector (.x _returnvalue_2) (.y _returnvalue_2) (+ (.z _returnvalue_2) (Variables|Default|GetDistanceAbovemesh))) false false)
  (if (Variables|Default|GetUpdateActor)
    (bind (_outhit _returnvalue_3) (Collision|LineTraceByChannel (Transformation|GetActorLocation) (Transformation|GetWorldLocation (Variables|/Game/GameBP/Level1/L1_Horror_Character.L1_Horror_Character_C|GetCamera (Variables|Default|GetPlayerREf))) "TraceTypeQuery1" false 0 "None"))
    (if _returnvalue_3
      (Rendering|SetVisibility _promptwidget false false)
      (Input|DisableInput (Game|GetPlayerController 0))
      (else
        (Rendering|SetVisibility _promptwidget true false)
        (Transformation|SetWorldRotation (Variables|Default|GetPromptWidget) (Math|Rotator|FindLookatRotation (Transformation|GetWorldLocation (Variables|Default|GetPromptWidget)) (Transformation|GetWorldLocation (Variables|/Game/GameBP/Level1/L1_Horror_Character.L1_Horror_Character_C|GetCamera (Variables|Default|GetPlayerREf)))) false false)
        (Default|TogglePrompt (.AsW%20%20Horror%20Pick%20Up%20Prompt (Utilities|Casting|CastToW__Horror_PickUp_Prompt (UserInterface|GetUserWidgetObject (Variables|Default|GetPromptWidget)))) (<= (Math|Vector|VectorLength (- (.TraceStart (Collision|BreakHitResult _outhit)) (.TraceEnd (Collision|BreakHitResult _outhit)))) (Variables|Default|GetPickUpDistance)))
        (if (<= (Math|Vector|VectorLength (- (.TraceStart (Collision|BreakHitResult _outhit)) (.TraceEnd (Collision|BreakHitResult _outhit)))) (Variables|Default|GetPickUpDistance))
          (Input|EnableInput _returnvalue)
          (else
            (Input|DisableInput _returnvalue)))))))

(event EventBeginPlay
  (bind _outactors (Actor|GetAllActorsOfClass "/Game/BP/Actors/Notes/BP_Note_Examination.BP_Note_Examination_C"))
  (Variables|Default|SetBP_Note_Exa_ref (Utilities|Array|Get(acopy) _outactors)))

(event Input|ActionEvents|InputActionAction
  (params (Key :type Key%20Structure :default "None"))
  (:Pressed
    (Utilities|IsValid (Variables|Default|GetW_Exam_Note_Ref)
      (:Is%20Not%20Valid
        (bind _returnvalue (UserInterface|CreateWidget "/Game/UMG/W_Horror_Note_Examine.W_Horror_Note_Examine_C" 0 0 (Variables|Default|GetBP_Note_Exa_ref)))
        (Variables|Default|SetW_Exam_Note_Ref _returnvalue)
        (Default|UpdateWidget _returnvalue self)
        (UserInterface|Viewport|AddtoViewport _returnvalue 0)))))

(fn ConstructionScript
  (Rendering|Components|TextRender|SetText (Variables|Default|GetNoteText) (Variables|Default|GetNote%20Text%28text%29))
  (Rendering|Components|TextRender|SetText (Variables|Default|GetBackNoteText) (Variables|Default|GetBack%20Note%20Text%28text%29)))