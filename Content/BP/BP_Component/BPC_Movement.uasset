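; Movement component for the horror game's player character, handling walk, stamina-limited sprint and crouch by setting the character's max walk speed.
; Looping timers called by function name drain stamina while sprinting and moving, then regenerate it after a retriggerable delay once sprint stops.
; Crouch cancels the sprint timer without scheduling regeneration and resizes the capsule through a cast to L1_Horror_Character.
; Initialize supplies the character reference.
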(event Custom|StartSprint
  ;[1 1 1] checkagem da stamina
  (if (Variables|Default|GetIsCrouching)
    (CallFunction|EndCrouch))
  (if (and (> (Variables|Default|GetCurrentStamina) (Variables|Default|GetMinStamina)) (> (Math|Vector|VectorLength (Transformation|GetVelocity (Variables|Default|GetPlayerRef))) 1e+01))
    (Utilities|Time|ClearTimerbyFunctionName 0 "Regenerate Stamina")
    (CallFunction|SetMaxWalkSpeed (Variables|Default|GetSprintSpeed))
    (Utilities|Time|SetTimerbyFunctionName 0 "SprintTimer" 1.0 true)))

(event Custom|SprintTimer
  ;[1 1 1] Gastar Stamina
  (if (> (Math|Vector|VectorLength (Transformation|GetVelocity (Variables|Default|GetPlayerRef))) 1e+01)
    (Variables|Default|SetCurrentStamina (Math|Float|Clamp(Float) (- (Variables|Default|GetCurrentStamina) 1.0) (Variables|Default|GetMinStamina) (Variables|Default|GetMaxStamina)))
    (if (<= (Variables|Default|GetCurrentStamina) (Variables|Default|GetMinStamina))
      (CallFunction|StopSprint))
    (else
      (CallFunction|StopSprint))))

(event Custom|StopSprint
  ;[1 1 1] Parar de correr
  (if (not (Variables|Default|GetIsCrouching))
    (Utilities|Time|ClearTimerbyFunctionName 0 "SprintTimer")
    (CallFunction|SetMaxWalkSpeed (Variables|Default|GetWalkSpeed))
    (Utilities|FlowControl|RetriggerableDelay 5.0)
    (if (not (Class|KismetSystemLibrary|IsTimerActive 0 "SprintTimer"))
      (Utilities|Time|SetTimerbyFunctionName 0 "Regenerate Stamina" 0.3 true))))

(event Custom|Regenerate%20Stamina
  ;[1 1 1] Regeneração de Stamina
  (Variables|Default|SetCurrentStamina (Math|Float|Clamp(Float) (+ (Variables|Default|GetCurrentStamina) 1.0) (Variables|Default|GetMinStamina) (Variables|Default|GetMaxStamina)))
  (if (>= (Variables|Default|GetCurrentStamina) (Variables|Default|GetMaxStamina))
    (Utilities|Time|ClearTimerbyFunctionName 0 "Regenerate Stamina")))

(event Custom|StartCrouch
  ;[1 1 1] Agachar
  (Utilities|Time|ClearTimerbyFunctionName 0 "SprintTimer")
  (CallFunction|SetMaxWalkSpeed (Variables|Default|GetCrouchSpeed))
  (Default|ShortenPlayerCapsule (.AsL1%20Horror%20Character (Utilities|Casting|CastToL1_Horror_Character (Variables|Default|GetPlayerRef))))
  (Variables|Default|SetIsCrouching true))

(event Custom|EndCrouch
  ;[1 1 1] Agachar
  (CallFunction|SetMaxWalkSpeed (Variables|Default|GetWalkSpeed))
  (Default|LenghtenCapsuleCapsule (.AsL1%20Horror%20Character (Utilities|Casting|CastToL1_Horror_Character (Variables|Default|GetPlayerRef))))
  (Variables|Default|SetIsCrouching false))

(fn Initialize
  (params (Character :type Character%20Object%20Reference))
  (Variables|Default|SetPlayerRef Character)
  (Variables|/Script/Engine.CharacterMovementComponent|SetMaxWalkSpeed (Variables|/Script/Engine.Character|GetCharacterMovement (Variables|Default|GetPlayerRef)) (Variables|Default|GetWalkSpeed)))

(fn SetMaxWalkSpeed
  (params (MaxWalkSpeed :type Float%20%28single-precision%29))
  (Variables|/Script/Engine.CharacterMovementComponent|SetMaxWalkSpeed (Variables|/Script/Engine.Character|GetCharacterMovement (Variables|Default|GetPlayerRef)) MaxWalkSpeed))