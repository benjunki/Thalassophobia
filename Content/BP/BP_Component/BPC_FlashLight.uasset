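; Actor component that gives the player a battery-powered flashlight.
; Initialize caches the player and its FlashLight component, whose visibility ToggleFlashLight flips, allowing it on only while charge is above the minimum.
; While lit, a looping timer drains the clamped battery and switches the light off at the minimum, avoiding Tick.
; AddBatteryLife restores charge within the same limits.
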(event EventBeginPlay)

(event EventTick
  (params (DeltaSeconds :type Float%20%28single-precision%29)))

(fn ToggleFlashLight
  (bind _flashlight_light (Variables|Default|GetFlashlight-Light))
  ;[1 1 1] Toggle da lanterna
  (if (Variables|/Script/Engine.SceneComponent|GetbVisible _flashlight_light)
    (Rendering|SetVisibility _flashlight_light false false)
    (Utilities|Time|ClearTimerbyFunctionName 0 "DepleteBatteryLife")
    (elif (> (Variables|Default|GetCurrentBattery) (Variables|Default|GetMinBattery))
      (Rendering|SetVisibility _flashlight_light true false)
      (Utilities|Time|SetTimerbyFunctionName 0 "DepleteBatteryLife" (Variables|Default|GetDepletionTIme) true))))

(fn Initialize
  (params (player :type L1%20Horror%20Character%20Object%20Reference))
  (bind _output_get (Variables|Default|SetPlayerRef player))
  (Variables|Default|SetFlashlight-Light (Variables|/Game/GameBP/Level1/L1_Horror_Character.L1_Horror_Character_C|GetFlashLight _output_get)))

(fn DepleteBatteryLife
  (Variables|Default|SetCurrentBattery (Math|Float|Clamp(Float) (- (Variables|Default|GetCurrentBattery) (Variables|Default|GetDepletionAmount)) (Variables|Default|GetMinBattery) (Variables|Default|GetMaxBattery)))
  (if (<= (Variables|Default|GetCurrentBattery) (Variables|Default|GetMinBattery))
    (Rendering|SetVisibility (Variables|Default|GetFlashlight-Light) false false)
    (Utilities|Time|ClearTimerbyFunctionName 0 "DepleteBatteryLife")))

(fn AddBatteryLife
  (params (Amount :type Float%20%28single-precision%29))
  (Variables|Default|SetCurrentBattery (Math|Float|Clamp(Float) (+ (Variables|Default|GetCurrentBattery) Amount) (Variables|Default|GetMinBattery) (Variables|Default|GetMaxBattery))))