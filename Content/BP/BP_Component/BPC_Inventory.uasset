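; Inventory component for a horror game that manages the player's item slots, sized from the player controller, and refreshes the inventory grid widget.
; AddItem recursively fills partial stacks, then empty slots, returning any remainder.
; UseItem calls the item actor, found or spawned, and consumes one on success; DropItem spawns a physics pickup at a camera trace.
; It also creates the examination widget and swaps it in over the inventory menu.
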(event Custom|Initialize
  (bind _returnvalue (Game|GetPlayerController 0))
  (bind _ashorror_player_controller (Utilities|Casting|CastToHorror_PlayerController _returnvalue))
  (Utilities|Array|Resize (Variables|Default|GetS_InventoryItem) (Variables|/Game/GameBP/Horror_PlayerController.Horror_PlayerController_C|GetInventorySlots _ashorror_player_controller))
  (Variables|Default|SetW%20Inventory%20Menu (Variables|/Game/GameBP/Horror_PlayerController.Horror_PlayerController_C|GetInventoryMenuRef _ashorror_player_controller))
  (bind _asl1_horror_character (Utilities|Casting|CastToL1_Horror_Character (Game|GetPlayerCharacter 0)))
  (Variables|Default|SetPlayer%20Ref _asl1_horror_character)
  (bind _returnvalue_2 (UserInterface|CreateWidget "/Game/UMG/Inventory/W_Horror_Examine.W_Horror_Examine_C" 0 0))
  (Variables|Default|SetW%20Examination%20Ref _returnvalue_2)
  (Variables|/Game/GameBP/Horror_PlayerController.Horror_PlayerController_C|SetW%20Exam%20Ref _ashorror_player_controller (Variables|Default|GetW%20Examination%20Ref))
  (bind _outactors (Actor|GetAllActorsOfClass "/Game/BP/Actors/Inventory/BP_Examination.BP_Examination_C"))
  (Variables|Default|SetBP%20Examination%20Ref (Utilities|Array|Get(acopy) _outactors))
  (Variables|/Game/UMG/Inventory/W_Horror_Examine.W_Horror_Examine_C|SetBPC%20Inventory%20Ref (Variables|Default|GetW%20Examination%20Ref) self))

(event Custom|CreateExaminationWidget
  (params (Index :type Integer))
  (bind _w_inventory_menu (Variables|Default|GetW%20Inventory%20Menu))
  (Default|UpdateWidget (Variables|Default|GetW%20Examination%20Ref) Index)
  (Widget|SetVisibility (Variables|Default|GetW%20Inventory%20Menu) "Collapsed")
  (Widget|SetVisibility _w_inventory_menu "Collapsed")
  (Utilities|IsValid (Variables|/Game/UMG/Inventory/W_Horror_InventoryMenu.W_Horror_InventoryMenu_C|GetW_Horror_InventoryDropDown _w_inventory_menu)
    (:Is%20Valid
      (Default|CloseDropDown _w_inventory_menu))
    (:Is%20Not%20Valid
      _))
  (UserInterface|Viewport|AddtoViewport (Variables|Default|GetW%20Examination%20Ref) 2)
  (Variables|/Game/GameBP/Horror_PlayerController.Horror_PlayerController_C|SetIsInventoryOpen (.AsHorror%20Player%20Controller (Utilities|Casting|CastToHorror_PlayerController (Game|GetPlayerController 0))) false))

(event EventBeginPlay
  (CallFunction|Initialize))

(event EventTick
  (params (DeltaSeconds :type Float%20%28single-precision%29)))

(fn AddItem
  (params (Item :type BP%20Inventory%20Item%20Master%20Class%20Reference) (Amount :type Integer))
  (bind (_sucess_ _index) (CallFunction|CheckforEmptySlot))
  (bind (_sucess__2 _index_2) (CallFunction|CheckforEmptySlot))
  (LocalVariables|SetLocalItem Item)
  (LocalVariables|SetLocalAmount Amount)
  (LocalVariables|SetLocalMaxStackAmount (.MaxStackAmount (Utilities|Struct|BreakS_ItemData (.S_ItemData (Utilities|GetClassDefaults (LocalVariables|GetLocalItem))))))
  (if (> (.MaxStackAmount (Utilities|Struct|BreakS_ItemData (.S_ItemData (Utilities|GetClassDefaults (LocalVariables|GetLocalItem))))) 1)
    (bind (_sucess__3 _index_3) (CallFunction|CheckforFreeSlot (LocalVariables|GetLocalItem)))
    (if _sucess__3
      (LocalVariables|SetLocalIndex _index_3)
      (if (> (+ (.Amount (CallFunction|GetItemDataatIndex (LocalVariables|GetLocalIndex))) (LocalVariables|GetLocalAmount)) (LocalVariables|GetLocalMaxStackAmount))
        (LocalVariables|SetLocalAmount (- (+ (.Amount (CallFunction|GetItemDataatIndex (LocalVariables|GetLocalIndex))) (LocalVariables|GetLocalAmount)) (LocalVariables|GetLocalMaxStackAmount)))
        (Utilities|Array|SetArrayElem (Variables|Default|GetS_InventoryItem) (LocalVariables|GetLocalIndex) (Utilities|Struct|MakeS_InventoryItems (LocalVariables|GetLocalItem) (LocalVariables|GetLocalMaxStackAmount)))
        (CallFunction|UpdateInventorySlot (LocalVariables|GetLocalIndex))
        (bind _remainder (CallFunction|AddItem (LocalVariables|GetLocalItem) (LocalVariables|GetLocalAmount)))
        (return true _remainder)
        (else
          (Utilities|Array|SetArrayElem (Variables|Default|GetS_InventoryItem) (LocalVariables|GetLocalIndex) (Utilities|Struct|MakeS_InventoryItems (LocalVariables|GetLocalItem) (+ (.Amount (CallFunction|GetItemDataatIndex (LocalVariables|GetLocalIndex))) (LocalVariables|GetLocalAmount))))
          (CallFunction|UpdateInventorySlot (LocalVariables|GetLocalIndex))
          (return true 0)))
      (elif _sucess_
        (LocalVariables|SetLocalIndex _index)
        (if (> (LocalVariables|GetLocalAmount) (LocalVariables|GetLocalMaxStackAmount))
          (Utilities|Array|SetArrayElem (Variables|Default|GetS_InventoryItem) (LocalVariables|GetLocalIndex) (Utilities|Struct|MakeS_InventoryItems (LocalVariables|GetLocalItem) (LocalVariables|GetLocalMaxStackAmount)))
          (CallFunction|UpdateInventorySlot (LocalVariables|GetLocalIndex))
          (bind _remainder_2 (CallFunction|AddItem (LocalVariables|GetLocalItem) (- (LocalVariables|GetLocalAmount) (LocalVariables|GetLocalMaxStackAmount))))
          (return true _remainder_2)
          (else
            (Utilities|Array|SetArrayElem (Variables|Default|GetS_InventoryItem) (LocalVariables|GetLocalIndex) (Utilities|Struct|MakeS_InventoryItems (LocalVariables|GetLocalItem) (LocalVariables|GetLocalAmount)))
            (CallFunction|UpdateInventorySlot (LocalVariables|GetLocalIndex))
            (return true 0)))
        (else
          (return false (LocalVariables|GetLocalAmount)))))
    (elif _sucess__2
      (LocalVariables|SetLocalIndex _index_2)
      (Utilities|Array|SetArrayElem (Variables|Default|GetS_InventoryItem) (LocalVariables|GetLocalIndex) (Utilities|Struct|MakeS_InventoryItems (LocalVariables|GetLocalItem) 1))
      (CallFunction|UpdateInventorySlot (LocalVariables|GetLocalIndex))
      (if (> (- (LocalVariables|GetLocalAmount) 1) 0)
        (bind _remainder_3 (CallFunction|AddItem (LocalVariables|GetLocalItem) (- (LocalVariables|GetLocalAmount) 1)))
        (return true _remainder_3)
        (else
          (return true 0)))
      (else
        (Development|PrintString "NofreeSlots")
        (return false (LocalVariables|GetLocalAmount))))))

(fn CheckforEmptySlot
  (bind (_array_element _array_index) (Utilities|Array|ForEachLoopwithBreak (Variables|Default|GetS_InventoryItem) :!label _label)
    (:LoopBody
      (if (Utilities|IsValidClass (.Item (Utilities|Struct|BreakS_InventoryItems _array_element)))
        (LocalVariables|SetLocalSucess false)
        (else
          (LocalVariables|SetLocalSucess true)
          (LocalVariables|SetLocalIndex _array_index)
          (goto _label Break))))
    (:Completed
      (return (LocalVariables|GetLocalSucess) (LocalVariables|GetLocalIndex)))))

(fn GetItemDataatIndex
  (params (Index :type Integer))
  (bind _s_inventoryitem (Variables|Default|GetS_InventoryItem))
  (bind _output (Utilities|Array|Get(acopy) _s_inventoryitem Index))
  (bind (_item _amount) (Utilities|Struct|BreakS_InventoryItems _output))
  (return _item _amount))

(fn UpdateInventorySlot
  (params (Index :type Integer))
  (Default|UpdateSlot (Utilities|Array|Get(acopy) (Variables|/Game/UMG/Inventory/W_Horror_InventoryGrid.W_Horror_InventoryGrid_C|GetSlotsArray (Variables|/Game/UMG/Inventory/W_Horror_InventoryMenu.W_Horror_InventoryMenu_C|GetW_Horror_InventoryGrid (Variables|/Game/GameBP/Horror_PlayerController.Horror_PlayerController_C|GetInventoryMenuRef (.AsHorror%20Player%20Controller (Utilities|Casting|CastToHorror_PlayerController (Game|GetPlayerController 0)))))) Index)))

(fn CheckforFreeSlot
  (params (item :type BP%20Inventory%20Item%20Master%20Class%20Reference))
  (bind (_array_element _array_index) (Utilities|Array|ForEachLoopwithBreak (Variables|Default|GetS_InventoryItem) :!label _label)
    (:LoopBody
      (if (and (== (.Item (Utilities|Struct|BreakS_InventoryItems _array_element)) item) (< (.Amount (Utilities|Struct|BreakS_InventoryItems _array_element)) (.maxstackamount (.S_ItemData (Utilities|GetClassDefaults item)))))
        (LocalVariables|SetLocalSucess true)
        (LocalVariables|SetLocalIndex _array_index)
        (goto _label Break)
        (else
          (LocalVariables|SetLocalSucess false))))
    (:Completed
      (return (LocalVariables|GetLocalSucess) (LocalVariables|GetLocalIndex)))))

(fn UseItem
  (params (Index :type Integer))
  (bind _output_get (LocalVariables|SetLocalIndex Index))
  (if (> (.Amount (CallFunction|GetItemDataatIndex _output_get)) 0)
    (bind _returnvalue (Actor|GetActorOfClass (.Item (CallFunction|GetItemDataatIndex _output_get))))
    (Utilities|IsValid _returnvalue
      (:Is%20Valid
        (Default|UseItem _returnvalue)
        (if (Variables|/Game/BP/Actors/Inventory/BP_InventoryItem_Master.BP_InventoryItem_Master_C|GetUseItemSucess _returnvalue)
          (CallFunction|RemoveItem (LocalVariables|GetLocalIndex) :!label _label)
          (Default|CloseDropDown (Variables|Default|GetW%20Inventory%20Menu))))
      (:Is%20Not%20Valid
        (bind _returnvalue_2 (Game|SpawnActorfromClass (.Item (CallFunction|GetItemDataatIndex _output_get)) (Math|Transform|MakeTransform "0, 0, 0" "0, 0, 0" "1,1,1") "Undefined" 0 0))
        (Default|UseItem _returnvalue_2)
        (if (Variables|/Game/BP/Actors/Inventory/BP_InventoryItem_Master.BP_InventoryItem_Master_C|GetUseItemSucess _returnvalue_2)
          (goto _label))))))

(fn RemoveItem
  (params (Index :type Integer))
  (LocalVariables|SetLocalIndex Index)
  (if (> (.Amount (CallFunction|GetItemDataatIndex (LocalVariables|GetLocalIndex))) 1)
    (Utilities|Array|SetArrayElem (Variables|Default|GetS_InventoryItem) (LocalVariables|GetLocalIndex) (Utilities|Struct|MakeS_InventoryItems (.Item (CallFunction|GetItemDataatIndex (LocalVariables|GetLocalIndex))) (- (.Amount (CallFunction|GetItemDataatIndex (LocalVariables|GetLocalIndex))) 1)))
    (else
      (Utilities|Array|SetArrayElem (Variables|Default|GetS_InventoryItem) (LocalVariables|GetLocalIndex) (Utilities|Struct|MakeS_InventoryItems 0 0))))
  (CallFunction|UpdateInventorySlot (LocalVariables|GetLocalIndex)))

(fn DropItem
  (params (Index :type Integer))
  (bind _player_ref (Variables|Default|GetPlayer%20Ref))
  (bind _camera (Variables|/Game/GameBP/Level1/L1_Horror_Character.L1_Horror_Character_C|GetCamera _player_ref))
  (bind _returnvalue (Transformation|GetWorldLocation _camera))
  (bind _output_get (LocalVariables|SetLocalIndex Index))
  (LocalVariables|SetLocalAmount (.Amount (CallFunction|GetItemDataatIndex _output_get)))
  (LocalVariables|SetLocalClassItem (.Item (CallFunction|GetItemDataatIndex _output_get)))
  (if (> (LocalVariables|GetLocalAmount) 0)
    (for _index (range 0 (- (LocalVariables|GetLocalAmount) 1))
      (CallFunction|RemoveItem (LocalVariables|GetLocalIndex)))
    (Default|CloseDropDown (Variables|Default|GetW%20Inventory%20Menu))
    ;[1 1 1] Fazer o item aparecer ao dropar
    (bind (_outhit _returnvalue_2) (Collision|LineTraceByChannel _returnvalue (+ _returnvalue (* (Math|Vector|GetForwardVector _camera) 2e+02)) "TraceTypeQuery1" false 0 "None"))
    (bind _returnvalue_3 (Game|SpawnActorfromClass (.PickUpActor (Utilities|Struct|BreakS_ItemData (.S_ItemData (Utilities|GetClassDefaults (LocalVariables|GetLocalClassItem))))) (Math|Transform|MakeTransform (select _returnvalue_2 (.Location (Collision|BreakHitResult _outhit)) (.TraceEnd (Collision|BreakHitResult _outhit))) "0, 0, 0" "1,1,1") "Undefined" 0 0))
    (Variables|/Game/BP/Actors/Inventory/PickUpActors/BP_PickupActor_Master.BP_PickupActor_Master_C|Setamount _returnvalue_3 (LocalVariables|GetLocalAmount))
    (Physics|SetSimulatePhysics (Variables|/Game/BP/Actors/Inventory/PickUpActors/BP_PickupActor_Master.BP_PickupActor_Master_C|GetStaticMesh _returnvalue_3) true)))